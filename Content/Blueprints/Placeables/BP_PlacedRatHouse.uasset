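; BP_PlacedRatHouse is a placeable rat spawner that keeps a limited rat population around itself.
; A looping timer started at BeginPlay periodically counts every BP_Rat within a set radius, using squared distance checks.
; While that count is below the cap, it spawns one rat at SpawnLocation, transformed from the house's local space, adjusting for collisions or skipping the spawn if blocked.
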(event `self.ReceiveBeginPlay`
  (`parent.ReceiveBeginPlay`)
  (`KismetSystemLibrary.K2_SetTimerDelegate` (delegate `TrySpawnRat`) 5.0 true))

(event `TrySpawnRat`
  (set `self.RatCount` 0)
  (bind _outactors (`GameplayStatics.GetAllActorsOfClass` "/Game/Blueprints/Character/Animals/Rat/BP_Rat.BP_Rat_C"))
  (for _array_element _outactors
    (if (<= (`self.GetSquaredDistanceTo` _array_element self) (`KismetMathLibrary.Square` 7500.0))
      (`/Engine/EditorBlueprintResources/StandardMacros.IncrementInt` (`self.RatCount`))))
  (if (< (`self.RatCount`) 7)
    (`|SpawnActorFromClass` "/Game/Blueprints/Character/Animals/Rat/BP_Rat.BP_Rat_C" (`KismetMathLibrary.MakeTransform` (`KismetMathLibrary.TransformLocation` (`self.GetTransform`) (`self.SpawnLocation`))) "AdjustIfPossibleButDontSpawnIfColliding" "OverrideRootScale" null null)))

(fn `UserConstructionScript`
  (`parent.UserConstructionScript`))