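; Base AI controller for animals that runs a behavior tree on the controlled BaseAnimal.
; On BeginPlay it sets up the assigned blackboard asset and starts the behavior tree.
; Every tick it mirrors the pawn's Hunger and Thirst into the blackboard.
; It also derives IsDead from Health and CanMove from being alive and not trapped, so the tree can react to them.
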(event `self.ReceiveBeginPlay`
  (bind _blackboardcomponent (`self.UseBlackboard` (`self.BlackboardAsset`)))
  (set `self.BB` _blackboardcomponent)
  (`self.RunBehaviorTree` (`self.BTAsset`)))

(event `self.ReceiveTick`
  (params (DeltaSeconds :type "Float (single-precision)"))
  (bind _asbase_animal (cast `BaseAnimal` (`self.K2_GetPawn`) :!pure true))
  (bind _returnvalue (<= (`BaseAnimal.Health` _asbase_animal) 0.0))
  (`BlackboardComponent.SetValueAsFloat` (`self.BB`) "Hunger" (`BaseAnimal.Hunger` (cast `BaseAnimal` (`self.K2_GetPawn`) :!pure true)))
  (`BlackboardComponent.SetValueAsFloat` (`self.BB`) "Thirst" (`BaseAnimal.Thirst` _asbase_animal))
  (`BlackboardComponent.SetValueAsBool` (`self.BB`) "IsDead" _returnvalue)
  (`BlackboardComponent.SetValueAsBool` (`self.BB`) "CanMove" (and (not _returnvalue) (not (`BaseAnimal.bIsTrapped` _asbase_animal)))))

(fn `UserConstructionScript`)