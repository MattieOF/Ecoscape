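; BP_TDCharacter is the player character Blueprint that handles tool selection for placing, painting and destroying objects and placing fences.
; Number keys 1 to 5 each pass a tool type to SetCurrentTool, including a no-tool option.
; The OnFailedPlacementAttempt event plays a 2D error sound, while the tool behavior itself is not implemented in this graph.
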(event `Key|One`
  (params (Key :type "Key Structure"))
  (:`Pressed`
    (`self.SetCurrentTool` "ETNone")))

(event `Key|Two`
  (params (Key :type "Key Structure"))
  (:`Pressed`
    (`self.SetCurrentTool` "ETPlaceObjects")))

(event `Key|Three`
  (params (Key :type "Key Structure"))
  (:`Pressed`
    (`self.SetCurrentTool` "ETPaintObjects")))

(event `Key|Four`
  (params (Key :type "Key Structure"))
  (:`Pressed`
    (`self.SetCurrentTool` "ETDestroyObjects")))

(event `Key|Five`
  (params (Key :type "Key Structure"))
  (:`Pressed`
    (`self.SetCurrentTool` "ETPlaceFence")))

(event `self.OnFailedPlacementAttempt`
  (`GameplayStatics.PlaySound2D` "/Engine/EditorSounds/Notifications/CompileFailed_Cue.CompileFailed_Cue" 1.0 1.0 0.0 null null))

(fn `UserConstructionScript`)