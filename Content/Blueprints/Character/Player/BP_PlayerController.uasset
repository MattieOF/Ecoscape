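; Player controller for Ecoscape that manages the first-person and top-down HUDs and reacts to player view changes.
; View changes hide both HUDs, time the character mesh's visibility, then after the transition show the matching HUD or play menu music.
; Hardcoded keys open the animal-naming widget (N), blend to the "Observation" camera (C), and spawn a panda under the cursor (P).
; The habitat-select widget and camera logic is unconnected.
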(event `self.SetupHUD`
  (bind _widget (`/Game/Blueprints/Utilities/BP_GeneralActorMacroLibrary.AddNewWidget` "/Game/UI/W_FirstPersonHUD.W_FirstPersonHUD_C"))
  (set `self.FirstPersonHUD` (cast `/Game/UI/W_FirstPersonHUD` _widget :!pure true))
  (bind _widget_2 (`/Game/Blueprints/Utilities/BP_GeneralActorMacroLibrary.AddNewWidget` "/Game/UI/W_TopDownHUD.W_TopDownHUD_C"))
  (set `self.TopDownHUD` (cast `/Game/UI/W_TopDownHUD` _widget_2 :!pure true)))

(event `self.OnEcoscapePlayerViewChanged`
  (params (NewState :type "EEcoscapePlayerView Enum" :default "EPSFirstPerson") (NewPawn :type "Pawn Object Reference") (Time :type "Float (single-precision)"))
  (`/Engine/EditorBlueprintResources/StandardMacros.IsValid` (`self.TopDownHUD`)
    (:`Is Valid`
      (`Widget.SetVisibility` (`self.TopDownHUD`) "Hidden")
      (`Widget.SetVisibility` (`self.FirstPersonHUD`) "Hidden")
      (`self.ChangePlayerModelVisibility` true 0.1)
      (switch `EEcoscapePlayerView` NewState
        (:`EPSFirstPerson`
          (`self.ChangePlayerModelVisibility` false (- Time 0.01)))
        (:`EPSTopDown`
          _)
        (:`EPSMenu`
          _))
      (`KismetSystemLibrary.Delay` Time)
      (switch `EEcoscapePlayerView` NewState
        (:`EPSFirstPerson`
          (`Widget.SetVisibility` (`self.FirstPersonHUD`) "SelfHitTestInvisible"))
        (:`EPSTopDown`
          (`Widget.SetVisibility` (`self.TopDownHUD`) "SelfHitTestInvisible"))
        (:`EPSMenu`
          (`self.PlayMusic` "/Game/Sound/Music/Menu.Menu"))))))

(event `ChangePlayerModelVisibility`
  (params (NewVisibility :type Boolean) (Time :type "Float (double-precision)"))
  (if (not (<= Time 0.0))
    (`KismetSystemLibrary.Delay` Time))
  (`SceneComponent.SetVisibility` (`/Game/Blueprints/Character/Player/BP_FPCharacter.CharacterMesh` (cast `/Game/Blueprints/Character/Player/BP_FPCharacter` (`self.FPCharacter`) :!pure true)) NewVisibility false))

(event `Key|N`
  (params (Key :type "Key Structure"))
  (:`Pressed`
    (bind _returnvalue (`|CreateWidget` "/Game/UI/W_NameAnimal.W_NameAnimal_C" null null))
    (`UserWidget.AddToViewport` _returnvalue 0)))

(event `Key|C`
  (params (Key :type "Key Structure"))
  (:`Pressed`
    (`self.SetViewTargetWithBlend` (`EcoscapeStatics.GetFirstActorWithTag` "Observation") 1.0 "VTBlend_Linear" 2.0)
    (`Widget.SetVisibility` (`self.TopDownHUD`) "Hidden")
    (`Widget.SetVisibility` (`self.FirstPersonHUD`) "Hidden")))

(event `Key|P`
  (params (Key :type "Key Structure"))
  (:`Pressed`
    (bind _hitresult (`EcoscapeStatics.GetHitResultAtCursorByChannel` self "ECC_GameTraceChannel3" false (`|MakeArray` null :!type "Actor Object Reference")))
    (`BaseAnimal.SpawnAnimal` "/Game/Blueprints/Character/Animals/Panda/ANIMAL_Panda.ANIMAL_Panda" (cast `EcoscapeTerrain` (`.HitActor` (`GameplayStatics.BreakHitResult` _hitresult)) :!pure true) (+ (`.ImpactPoint` (`GameplayStatics.BreakHitResult` _hitresult)) (0.0 0.0 100.0)))))

(fn `UserConstructionScript`)