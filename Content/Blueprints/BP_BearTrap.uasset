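; BP_BearTrap is a single-use bear trap that snares animals or hurts the player.
; On overlap it plays its snap animation and sound, then destroys its trigger.
; A BaseAnimal is immobilized with happiness overridden to zero, while the player only gets a pain sound and W_Pain widget.
; Interacting runs a timeline that moves the trap vertically, then restores any trapped animal and destroys the trap.
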(event `self.ReceiveBeginPlay`
  (set `self.Original` (`self.K2_GetActorLocation`)))

(event `self.Trigger.OnComponentBeginOverlap`
  (params (OverlappedComponent :type "PrimitiveComponent Object Reference") (OtherActor :type "Actor Object Reference") (OtherComp :type "PrimitiveComponent Object Reference") (OtherBodyIndex :type Integer) (bFromSweep :type Boolean) (SweepResult :type "HitResult Structure (by ref)"))
  (`/Engine/EditorBlueprintResources/StandardMacros.IsValid` (`self.Trigger`)
    (:`Is Valid`
      (bind _asbase_animal (cast `BaseAnimal` OtherActor)
        (:`then`
          (bind _output_get (set `self.TrappedAnimal` _asbase_animal))
          (set `BaseAnimal.HappinessOverride` 0.0 _output_get)
          (set `BaseAnimal.bHasHappinessOverride` true _output_get)
          (set `BaseAnimal.bIsTrapped` true _output_get)
          (set `CharacterMovementComponent.MaxWalkSpeed` 0.0 (`Character.CharacterMovement` _output_get))
          (`SkeletalMeshComponent.Play` (`self.SkeletalMesh`) false)
          (`GameplayStatics.PlaySoundAtLocation` "/Game/Sound/SFX/Objects/SND_BearTrap_Cue.SND_BearTrap_Cue" (`self.K2_GetActorLocation`) (struct) 1.0 1.0 0.0 null null null null)
          (`ActorComponent.K2_DestroyComponent` (`self.Trigger`)))
        (:`CastFailed`
          (cast `/Game/Blueprints/Character/Player/BP_FPCharacter` OtherActor)
          (`SkeletalMeshComponent.Play` (`self.SkeletalMesh`) false)
          (`GameplayStatics.PlaySoundAtLocation` "/Game/Sound/SFX/Objects/SND_BearTrap_Cue.SND_BearTrap_Cue" (`self.K2_GetActorLocation`) (struct) 1.0 1.0 0.0 null null null null)
          (`GameplayStatics.PlaySoundAtLocation` "/Game/Sound/SFX/Animals/SND_Ow_Cue.SND_Ow_Cue" (`self.K2_GetActorLocation`) (struct) 1.0 1.0 0.0 null null null null)
          (bind _returnvalue (`|CreateWidget` "/Game/UI/W_Pain.W_Pain_C"))
          (`UserWidget.AddToViewport` _returnvalue 0)
          (`ActorComponent.K2_DestroyComponent` (`self.Trigger`)))))))

(event `self.Interactable.OnInteractedWith`
  (bind _trappedanimal (`self.TrappedAnimal`))
  (bind (_direction _z) (`Timeline|DisappearTimeline`)
    (:`Update`
      (`self.K2_SetActorLocation` (+ (`self.Original`) (`KismetMathLibrary.MakeVector` 0.0 0.0 _z))))
    (:`Finished`
      (`/Engine/EditorBlueprintResources/StandardMacros.IsValid` _trappedanimal
        (:`Is Valid`
          (set `BaseAnimal.HappinessOverride` 0.0 _trappedanimal)
          (set `BaseAnimal.bHasHappinessOverride` false _trappedanimal)
          (set `BaseAnimal.bIsTrapped` false _trappedanimal)
          (set `CharacterMovementComponent.MaxWalkSpeed` (`AnimalData.MoveSpeed` (`BaseAnimal.AnimalData` _trappedanimal)) (`Character.CharacterMovement` _trappedanimal)))
        (:`Is Not Valid`
          _))
      (`self.K2_DestroyActor`))))

(fn `UserConstructionScript`)